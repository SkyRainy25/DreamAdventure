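; Base enemy Blueprint handling spawn and dissolve visuals, motion-warp facing, loot drops and gold rewards.
; Timelines scale the mesh in on BeginPlay and drive "Dissolve" parameters on body and weapon materials.
; SpawnLoot rolls loot tier items and places them on evenly spaced rotations at random distances, using a one-shot timer and passing enemy level to DreamEffectActor drops.
; Destruction awards gold to the player character.
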(event `self.ReceiveBeginPlay`
  (bind (_direction `_새_트랙_0`) (`Timeline|SpawnTimeline`)
    (:`Update`
      (`SceneComponent.SetRelativeScale3D` (`self.Mesh`) (`KismetMathLibrary.MakeVector` `_새_트랙_0` `_새_트랙_0` `_새_트랙_0`)))))

(event `CombatInterface.UpdateFacingTarget`
  (params (Target :type "Vector Structure (by ref)"))
  (`MotionWarpingComponent.AddOrUpdateWarpTargetFromLocation` (`self.MotionWarping`) "FacingTarget" Target))

(event `self.StartDissolveTimeline`
  (params (DynamicMaterialInstance :type "MaterialInstanceDynamic Object Reference"))
  (bind (_direction `_새_트랙_0`) (`Timeline|Dissolve`)
    (:`Update`
      (`MaterialInstanceDynamic.SetScalarParameterValue` DynamicMaterialInstance "Dissolve" `_새_트랙_0`))))

(event `self.StartWeaponDissolveTimeline`
  (params (DynamicMaterialInstance :type "MaterialInstanceDynamic Object Reference"))
  (bind (_direction `_새_트랙_0`) (`Timeline|WeaponDissolve`)
    (:`Update`
      (`MaterialInstanceDynamic.SetScalarParameterValue` DynamicMaterialInstance "Dissolve" `_새_트랙_0`))))

(event `self.SpawnLoot`
  (bind _returnvalue (`DreamAbilitySystemLibrary.GetLootTiers` null))
  (`/Engine/EditorBlueprintResources/StandardMacros.IsValid` _returnvalue
    (:`Is Valid`
      (bind _returnvalue_2 (`LootTiers.GetLootItems` _returnvalue))
      (bind _output_get (set `self.LootItems` _returnvalue_2))
      (set `self.LootRotation` (`self.GetLootRotation` _output_get))
      (set `self.SpawnLootCount` 0)
      (bind _returnvalue_3 (`KismetSystemLibrary.K2_SetTimerDelegate` (delegate `SpawnLootItem`) 0.1))
      (set `self.LootTimer` _returnvalue_3)
      (`self.SpawnLootItem`))))

(event `SpawnLootItem`
  (bind (_lootclass _blootleveloverride) (break `LootItem` (`|GetArrayItem` (`self.LootItems`) (`self.SpawnLootCount`))))
  (if (< (`self.SpawnLootCount`) (`KismetArrayLibrary.Array_Length` (`self.LootItems`)))
    (bind _returnvalue (`|SpawnActorFromClass` _lootclass (`self.GetLootTransform` (`self.SpawnLootCount`)) "AlwaysSpawn" "MultiplyWithRoot" null null))
    (bind _asdream_effect_actor (cast `DreamEffectActor` _returnvalue))
    (`/Engine/EditorBlueprintResources/StandardMacros.IsValid` _asdream_effect_actor
      (:`Is Valid`
        (set `DreamEffectActor.ActorLevel` (`KismetMathLibrary.Conv_IntToDouble` (`self.Level`)) _asdream_effect_actor))
      (:`Is Not Valid`
        _))
    (`/Engine/EditorBlueprintResources/StandardMacros.IncrementInt` (`self.SpawnLootCount`)
      (:`  `
        (if _blootleveloverride
          _)))
    (else
      (`KismetSystemLibrary.K2_ClearAndInvalidateTimerHandle` (`self.LootTimer`)))))

(event `self.ReceiveDestroyed`
  (bind _asplayer_character (cast `PlayerCharacter` (`GameplayStatics.GetPlayerCharacter` 0)))
  (`DreamAbilitySystemLibrary.AddGold` _asplayer_character null (`self.Gold`)))

(fn `GetLootRotation`
  (params (TargetArray :type "Array of LootItem Structure (by ref)"))
  (returns (ReturnValue :type "Array of Rotator Structure"))
  (return (`DreamAbilitySystemLibrary.EvenlySpacedRotators` (`self.GetActorForwardVector`) (`KismetMathLibrary.Vector_Up`) 360.0 (`KismetArrayLibrary.Array_Length` TargetArray))))

(fn `GetLootTransform`
  (params (LootCount :type Integer))
  (returns (Transform :type "Transform Structure"))
  (bind _output (`|GetArrayItem` (`self.LootRotation`) LootCount))
  (return (`KismetMathLibrary.MakeTransform` (+ (* (`KismetMathLibrary.GetForwardVector` _output) (`KismetMathLibrary.RandomFloatInRange` (`self.MinSpawnDistance`) (`self.MaxSpawnDistance`))) (`self.K2_GetActorLocation`)) _output)))

(fn `UserConstructionScript`)