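; Store NPC that opens and closes a shop menu when the player interacts with G inside its collision box.
; Overlap creates an interaction key widget and binds to its click event, which toggles the StoreWidgetClass menu.
; On opening, it removes the prompt and calls OnOverlap with the player and ItemPackage.
; Leaving the box removes any open menu or prompt and unbinds the G key.
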(event `self.Box Collision.OnComponentBeginOverlap`
  (params (OverlappedComponent :type "PrimitiveComponent Object Reference") (OtherActor :type "Actor Object Reference") (OtherComp :type "PrimitiveComponent Object Reference") (OtherBodyIndex :type Integer) (bFromSweep :type Boolean) (SweepResult :type "HitResult Structure (by ref)"))
  (bind _asplayer_character (cast `PlayerCharacter` OtherActor))
  (set `self.Player Character` _asplayer_character)
  ;[1 1 1] 상호작용 위젯 표시
  (bind _returnvalue (`|CreateWidget` "/Game/A_Game/Blueprints/UI/Interaction/WBP_InteractionKey_Screen.WBP_InteractionKey_Screen_C" (`GameplayStatics.GetPlayerController` 0)))
  (bind _output_get (set `self.InteractionWidget` _returnvalue))
  ;[1 1 1] 상호작용이 뜨고 G 클릭시 호출
  (`UserWidget.AddToViewport` _output_get 0)
  (add `/Game/A_Game/Blueprints/UI/Interaction/WBP_InteractionKey_Screen.InteractionKeyClicked` (`self.InteractionWidget`) (delegate `InteractionKeyClicked_이벤트`)))

(event `InteractionKeyClicked_이벤트`
  (params (Clicked :type Boolean))
  (bind _interactionwidget (`self.InteractionWidget`))
  (if Clicked
    ;[1 1 1] 창이 열렸는지
    (if (not (`self.IsOpen`))
      ;[1 1 1] 상점이 아직 열리지 않은 상태 + '상호작용'이 뜨고 처음 G Click
      (bind _returnvalue (`|CreateWidget` (`self.StoreWidgetClass`) (`GameplayStatics.GetPlayerController` 0)))
      (bind _output_get (set `self.StoreMenu` _returnvalue))
      (`UserWidget.AddToViewport` _output_get 0)
      ;[1 1 1] Display StoreMenu
      (`UserWidget.SetPositionInViewport` (`self.StoreMenu`) (100.0 100.0) true)
      (`/Engine/EditorBlueprintResources/StandardMacros.IsValid` _interactionwidget
        (:`Is Valid`
          (`Widget.RemoveFromParent` _interactionwidget)
          (set `self.IsOpen` true)
          (`self.OnOverlap` (`self.Player Character`) (`self.ItemPackage`)))))
    (else
      ;[1 1 1] 상점창이 열린 상태(IsOpen = true) + G 한번 더 클릭(false)
      (if (`self.IsOpen`)
        (`Widget.RemoveFromParent` (`self.StoreMenu`))
        ;[1 1 1] 충돌 영역을 벗어나면 G Key 를 통해 Menu를 못열도록 설정
        (set `self.IsOpen` false)
        (`/Game/A_Game/Blueprints/UI/Interaction/WBP_InteractionKey_Screen.UnBindGKey` (`self.InteractionWidget`))))))

(event `self.Box Collision.OnComponentEndOverlap`
  (params (OverlappedComponent :type "PrimitiveComponent Object Reference") (OtherActor :type "Actor Object Reference") (OtherComp :type "PrimitiveComponent Object Reference") (OtherBodyIndex :type Integer))
  (bind _storemenu (`self.StoreMenu`))
  (if (`self.IsOpen`)
    ;[1 1 1] Remove StoreMenu
    (`/Engine/EditorBlueprintResources/StandardMacros.IsValid` _storemenu
      (:`Is Valid`
        (`Widget.RemoveFromParent` _storemenu))))
  ;[1 1 1] InteractionKey_Screen이 화면에 있으면 제거
  (`/Engine/EditorBlueprintResources/StandardMacros.IsValid` (`self.InteractionWidget`)
    (:`Is Valid`
      (`Widget.RemoveFromParent` (`self.InteractionWidget`))
      (set `self.IsOpen` false)
      (`/Game/A_Game/Blueprints/UI/Interaction/WBP_InteractionKey_Screen.UnBindGKey` (`self.InteractionWidget`)))))

(fn `UserConstructionScript`)