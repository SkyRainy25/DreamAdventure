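; BP_FadeActor is an actor that fades its mesh and toggles its collision, running a fade-out then a delayed fade-in on BeginPlay.
; The construction script caches original materials and creates dynamic instances from fade materials.
; FadeOut applies those instances and plays a timeline driving their "Fade" parameter; FadeIn reverses it.
; FadeFinished restores materials and blocking at full value, or ignores a custom channel and optionally Visibility at zero.
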(event `/Game/A_Game/Blueprints/Actor/FadeActor/BI_FadeInterface.FadeOut`
  (`self.SetMaterialstoDynamicInstances`)
  (bind (_direction `_새_트랙_0`) (`Timeline|FadeTimeline` :!via `PlayFromStart` :!label _label)
    (:`Update`
      (for _array_element (`self.DynamicMaterialInstances`)
        (`MaterialInstanceDynamic.SetScalarParameterValue` _array_element "Fade" `_새_트랙_0`)))
    (:`Finished`
      (`self.FadeFinished` `_새_트랙_0`))))

(event `/Game/A_Game/Blueprints/Actor/FadeActor/BI_FadeInterface.FadeIn`
  (goto _label :!via `Reverse`))

(event `self.ReceiveBeginPlay`
  (`self.FadeOut`)
  (`KismetSystemLibrary.Delay` 1.0)
  (`self.FadeIn`))

(fn `FadeFinished`
  (params (InputPin :type "Float (single-precision)"))
  (if (>= InputPin 1.0)
    (`self.ReSetMaterials`)
    (`PrimitiveComponent.SetCollisionResponseToChannel` (`self.Mesh`) "ECC_GameTraceChannel2" "ECR_Block")
    ;[1 1 1] BlockVisibility = true? -> 이동 가능
    (if (`self.BlockVisibility`)
      (`PrimitiveComponent.SetCollisionResponseToChannel` (`self.Mesh`) "ECC_Visibility" "ECR_Block"))
    (elif (<= InputPin 0.0)
      (`PrimitiveComponent.SetCollisionResponseToChannel` (`self.Mesh`) "ECC_GameTraceChannel2" "ECR_Ignore")
      ;[1 1 1] BlockVisibility = true? -> 이동 가능
      (if (`self.BlockVisibility`)
        (`PrimitiveComponent.SetCollisionResponseToChannel` (`self.Mesh`) "ECC_Visibility" "ECR_Ignore")))))

(fn `ReSetMaterials`
  (for (_array_element _array_index) (`self.Original Materials`)
    (`PrimitiveComponent.SetMaterial` (`self.Mesh`) _array_index _array_element)))

(fn `SetMaterialstoDynamicInstances`
  (for (_array_element _array_index) (`self.DynamicMaterialInstances`)
    (`PrimitiveComponent.SetMaterial` (`self.Mesh`) _array_index _array_element)))

(fn `UserConstructionScript`
  (`KismetArrayLibrary.Array_Clear` (`self.DynamicMaterialInstances`))
  (set `self.Original Materials` (`MeshComponent.GetMaterials` (`self.Mesh`)))
  (for _array_element (`self.FadeMaterialInstances`)
    (bind _returnvalue (`KismetMaterialLibrary.CreateDynamicMaterialInstance` _array_element))
    (`KismetArrayLibrary.Array_AddUnique` (`self.DynamicMaterialInstances`) _returnvalue)))