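; BP_Pickup_Base is a base pickup actor that plays an elevation animation and sounds on spawn, then a consume sound when destroyed.
; A timeline drives CalculateElevation, which adds InitialLocation twice plus a SpawnApex-scaled height, and triggers a one-time impact sound above 0.8.
; When the timeline finishes, it starts sinusoidal movement and rotation.
; Tick applies the calculated location and rotation; overlap has no logic.
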(event `self.ReceiveBeginPlay`
  (`GameplayStatics.PlaySoundAtLocation` (`self.SpawnSound`) (`self.K2_GetActorLocation`) (struct) 1.0 1.0 0.0 null null null null)
  (bind (_direction _elevation) (`Timeline|PickupElevationTimeLine`)
    (:`Update`
      (set `self.Elevation` _elevation)
      (set `self.CalculatedLocation` (`self.CalculateElevation` (`self.Elevation`)))
      (if (> (`self.Elevation`) 0.8)
        (`/Engine/EditorBlueprintResources/StandardMacros.DoOnce` false
          (:`Completed`
            (`GameplayStatics.PlaySoundAtLocation` (`self.GroundImpactSound`) (`self.K2_GetActorLocation`) (struct) 1.0 1.0 0.0 null null null null)))))
    (:`Finished`
      (`self.StartSinusoidalMovement`)
      (`self.StartRotation`))))

(event `self.ReceiveTick`
  (params (DeltaSeconds :type "Float (single-precision)"))
  (`self.K2_SetActorLocation` (`self.CalculatedLocation`))
  (`self.K2_SetActorRotation` (`self.CalculatedRotation`)))

(event `self.ReceiveDestroyed`
  (`GameplayStatics.PlaySoundAtLocation` (`self.ConsumeSound`) (`self.K2_GetActorLocation`) (struct) 1.0 1.0 0.0 null null null null))

(fn `CalculateElevation`
  (params (A :type "Float (double-precision)"))
  (returns (ReturnValue :type "Vector Structure"))
  (bind _initiallocation (`self.InitialLocation`))
  (return (+ _initiallocation (`KismetMathLibrary.MakeVector` (.x _initiallocation) (.y _initiallocation) (+ (.z _initiallocation) (* A (`self.SpawnApex`)))))))

(fn `UserConstructionScript`)