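; BP_Torch is a torch actor whose fire light flickers continuously during play.
; On BeginPlay it randomly picks one of two flame intensity timelines and plays it from the start.
; Each timeline update sets the FireLight intensity to the curve value multiplied by BaseIntensity.
; When a timeline finishes, it picks again at random, so the flicker loops with varied patterns.
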(event `self.ReceiveBeginPlay`
  (`self.ChooseTimeline`))

(event `ChooseTimeline`
  (switch `int` (`KismetMathLibrary.RandomIntegerInRange` 0 1)
    (:`Default`
      (`self.StartTimeline_2` :!label _label))
    (:`0`
      (`self.StartTimeLine_1`))
    (:`1`
      (goto _label))))

(event `StartTimeLine_1`
  (bind (_direction _intensity) (`Timeline|FlameIntensityTimeline_1` :!via `PlayFromStart`)
    (:`Update`
      (`self.Scale FireIntensity` _intensity))
    (:`Finished`
      (`self.ChooseTimeline`))))

(event `StartTimeline_2`
  (bind (_direction _intensity) (`Timeline|FlameIntensityTimeline_2` :!via `PlayFromStart`)
    (:`Update`
      (`self.Scale FireIntensity` _intensity))
    (:`Finished`
      (`self.ChooseTimeline`))))

(fn `Scale FireIntensity`
  (params (A :type "Float (double-precision)"))
  (`LightComponent.SetIntensity` (`self.FireLight`) (* A (`self.BaseIntensity`))))

(fn `UserConstructionScript`)