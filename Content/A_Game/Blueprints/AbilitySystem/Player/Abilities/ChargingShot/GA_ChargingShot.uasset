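; Player gameplay ability for a held charging shot: a channeled shock beam aimed under the mouse that chains to additional targets.
; A montage event locks movement, adds looping beam GameplayCues and starts a timer that commits cost and deals magical damage.
; Release after a minimum skill time, unpaid cost or primary target death ends it, removing cues, applying server-side damage effects and committing cooldown.
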(event `self.K2_ActivateAbility`
  (`self.EnforceImplementsCombatInterface`)
  ;[1 1 1] Store Mouse Data Variables
  (bind (_asynctaskproxy _datahandle) (`TargetDataUnderMouse.CreateTargetDataUnderMouse`)
    (:`ValidData`
      (`self.StoreMouseDataInfo` (`AbilitySystemBlueprintLibrary.GetHitResultFromTargetData` _datahandle))
      (`self.StoreOwnerVariables`)
      (`|ExecutionSequence`
        (:`then_0`
          (set `PlayerController.bShowMouseCursor` false (`self.OwnerPlayerController`))
          (`self.UpdateFacingTarget`)
          (`self.K2_ExecuteGameplayCue` (struct :`TagName` "GameplayCue.ChargingShot"))
          (`AbilityTask_PlayMontageAndWait.CreatePlayMontageAndWaitProxy` "None" (`self.Montage_Charging`)
            (:`then`
              (`AbilityTask_WaitGameplayEvent.WaitGameplayEvent` (struct :`TagName` "Event.Montage.ChargingShot") null true
                (:`EventReceived`
                  (`self.InChargingLoop`)
                  (`self.SpawnChargingBeam`)
                  (bind _returnvalue (`KismetSystemLibrary.K2_SetTimerDelegate` (delegate `Damage And Cost`) (`self.DamageDeltaTime`) true))
                  (set `self.DamageAndCostTimer` _returnvalue))))))
        (:`then_1`
          ;[1 1 1] Enforce Minimum Skill Time
          (bind (_asynctaskproxy_2 _timeheld) (`AbilityTask_WaitInputRelease.WaitInputRelease` false)
            (:`OnRelease`
              (bind _output_get (set `self.Time Held` _timeheld))
              (if (< _output_get (`self.MinSkillTime`))
                (`self.K2_HasAuthority`
                  (:`True`
                    (`KismetSystemLibrary.Delay` (- (`self.MinSkillTime`) (`self.Time Held`)))
                    (`self.ClearTimerAndEndAbility` :!label _label))
                  (:`False`
                    (`self.PrepareForEndAbility`)))
                (else
                  (goto _label))))))))))

(event `Damage And Cost`
  (bind _returnvalue (`self.K2_CommitAbilityCost` false))
  (if _returnvalue
    (`self.ApplyDamage`)
    (else
      (`self.ClearTimerAndEndAbility`))))

(event `self.PrimaryTargetDied`
  (params (DeadActor :type "Actor Object Reference"))
  ;[1 0.1316 0] PrimaryTargetDied
  (`GameplayCueFunctionLibrary.RemoveGameplayCueOnActor` DeadActor (struct :`TagName` "GameplayCue.ChargingLoop") (`self.FirstTargetCueParams`))
  (`self.K2_CommitAbilityCooldown` false)
  (`self.ClearTimerAndEndAbility`))

(event `self.AdditionalTargetDied`
  (params (DeadActor :type "Actor Object Reference"))
  ;[1 0.1702 0] Additional Target Died. Remove Additional Targets and Additional ChargingLoop Cue
  (`self.Remove Charging Loop Cue from Additional Target` DeadActor)
  (`KismetArrayLibrary.Array_RemoveItem` (`self.Additional Targets`) DeadActor))

(fn `AddChargingLoopCueToAddtionalTarget`
  (params (AdditionalTarget :type "Actor Object Reference"))
  (locals (TargetActor :type "Actor Object Reference"))
  (bind _targetactor (`local.TargetActor`))
  (bind _returnvalue (`AbilitySystemBlueprintLibrary.MakeGameplayCueParameters` 0.0 0.0 (struct) (struct) (struct) (struct) (struct) (`Actor.K2_GetActorLocation` _targetactor) (0.0 0.0 0.0) null null _targetactor null 1 1 (`Actor.RootComponent` (`self.MouseHitActor`))))
  (set `local.TargetActor` AdditionalTarget)
  (`BlueprintMapLibrary.Map_Add` (`self.AdditionalActorsToCueParams`) (`local.TargetActor`) _returnvalue)
  (`GameplayCueFunctionLibrary.AddGameplayCueOnActor` (`local.TargetActor`) (struct :`TagName` "GameplayCue.ChargingLoop") _returnvalue))

(fn `ApplyDamage`
  (`self.ApplyDamageToSingleTarget` (`self.MouseHitActor`))
  (for _array_element (`self.Additional Targets`)
    (`self.ApplyDamageToSingleTarget` _array_element)))

(fn `ApplyDamageToSingleTarget`
  (params (Actor :type "Actor Object Reference"))
  (locals (DamageTarget :type "Actor Object Reference") (ASC :type "AbilitySystemComponent Object Reference"))
  (bind _returnvalue (`self.GetAbilitySystemComponentFromActorInfo`))
  (bind _returnvalue_2 (`AbilitySystemBlueprintLibrary.GetAbilitySystemComponent` (`local.DamageTarget`)))
  (bind _output_get (set `local.DamageTarget` Actor))
  (`/Engine/EditorBlueprintResources/StandardMacros.IsValid` _output_get
    (:`Is Valid`
      (bind _output_get_2 (set `local.ASC` _returnvalue))
      (`/Engine/EditorBlueprintResources/StandardMacros.IsValid` _output_get_2
        (:`Is Valid`
          (bind _returnvalue_3 (`AbilitySystemBlueprintLibrary.AssignTagSetByCallerMagnitude` (`AbilitySystemComponent.MakeOutgoingSpec` (`local.ASC`) (`self.DamageEffectClass`) (`KismetMathLibrary.Conv_IntToDouble` (`self.GetAbilityLevel`)) (`AbilitySystemComponent.MakeEffectContext` _returnvalue)) (struct :`TagName` "Damage.Magical") (`self.GetDamageAtLevel`)))
          (`/Engine/EditorBlueprintResources/StandardMacros.IsValid` _returnvalue_2
            (:`Is Valid`
              (`AbilitySystemComponent.BP_ApplyGameplayEffectSpecToSelf` _returnvalue_2 _returnvalue_3))))))))

(fn `ClearTimerAndEndAbility`
  (`KismetSystemLibrary.K2_ClearAndInvalidateTimerHandle` (`self.DamageAndCostTimer`))
  (`self.PrepareForEndAbility`)
  (`self.K2_CommitAbilityCooldown` false)
  (`KismetArrayLibrary.Array_Clear` (`self.Additional Targets`))
  (`BlueprintMapLibrary.Map_Clear` (`self.AdditionalActorsToCueParams`))
  (set `self.MouseHitActor` null)
  (set `self.FirstTargetImplementsInterface` false)
  (set `self.Time Held` 0.0)
  (`self.K2_EndAbility`))

(fn `EnforceImplementsCombatInterface`
  (if (not (`KismetSystemLibrary.DoesImplementInterface` (`self.GetAvatarActorFromActorInfo`) "/Script/DreamAdventure.CombatInterface"))
    (`self.K2_EndAbility`)))

(fn `InChargingLoop`
  (message `CombatInterface.SetInCharging` (`self.GetAvatarActorFromActorInfo`) true)
  (`CharacterMovementComponent.DisableMovement` (`Character.CharacterMovement` (`self.OwnerCharacter`))))

(fn `PrepareForEndAbility`
  (bind _mousehitactor (`self.MouseHitActor`))
  (set `PlayerController.bShowMouseCursor` true (`self.OwnerPlayerController`))
  (message `CombatInterface.SetInCharging` (`self.GetAvatarActorFromActorInfo`) false)
  (`CharacterMovementComponent.SetMovementMode` (`Character.CharacterMovement` (`self.OwnerCharacter`)) "MOVE_Walking" 0)
  (if (`self.FirstTargetImplementsInterface`)
    ;[1 1 1] Case : CombatInterface
    (message `CombatInterface.SetIsBeingShocked` _mousehitactor false)
    (`GameplayCueFunctionLibrary.RemoveGameplayCueOnActor` _mousehitactor (struct :`TagName` "GameplayCue.ChargingLoop") (`self.FirstTargetCueParams`))
    (`self.K2_HasAuthority`
      (:`True`
        (`DreamAbilitySystemLibrary.ApplyDamageEffect` (`self.MakeDamageEffectParamsFromClassDefaults` _mousehitactor)))
      (:`False`
        _))
    (for _array_element (`self.Additional Targets`)
      (message `CombatInterface.SetIsBeingShocked` _array_element false)
      (`self.Remove Charging Loop Cue from Additional Target` _array_element)
      (`self.K2_HasAuthority`
        (:`True`
          (`DreamAbilitySystemLibrary.ApplyDamageEffect` (`self.MakeDamageEffectParamsFromClassDefaults` _array_element)))))
    (else
      ;[1 1 1] Case : Wall or Floor .etc for reusing GameplayCue
      (`GameplayCueFunctionLibrary.RemoveGameplayCueOnActor` (`self.GetAvatarActorFromActorInfo`) (struct :`TagName` "GameplayCue.ChargingLoop") (`self.FirstTargetCueParams`)))))

(fn `Remove Charging Loop Cue from Additional Target`
  (params (AddtionalTarget :type "Actor Object Reference"))
  (locals (Target :type "Actor Object Reference"))
  (bind (_value _returnvalue) (`BlueprintMapLibrary.Map_Find` (`self.AdditionalActorsToCueParams`) (`local.Target`)))
  (set `local.Target` AddtionalTarget)
  (if _returnvalue
    (`GameplayCueFunctionLibrary.RemoveGameplayCueOnActor` (`local.Target`) (struct :`TagName` "GameplayCue.ChargingLoop") _value)))

(fn `SpawnChargingBeam`
  (locals (CueTarget :type "Actor Object Reference"))
  (`self.TraceFirstTarget` (`self.MouseHitLocation`))
  (bind _returnvalue (message `CombatInterface.GetStaticWeapon` (`self.OwnerCharacter`)))
  (set `self.FirstTargetCueParams` (`AbilitySystemBlueprintLibrary.MakeGameplayCueParameters` 0.0 0.0 (struct) (struct) (struct) (struct) (struct) (`self.MouseHitLocation`) (0.0 0.0 0.0) null null (`self.MouseHitActor`) null 1 1 _returnvalue))
  ;[1 1 1] Is Mouse HitActor Enemy?
  (bind _output_get (set `self.FirstTargetImplementsInterface` (`KismetSystemLibrary.DoesImplementInterface` (`self.MouseHitActor`) "/Script/DreamAdventure.CombatInterface")))
  (if _output_get
    ;[1 1 1] CombatInterface => Enemy
    (set `local.CueTarget` (`self.MouseHitActor`))
    (else
      ;[1 1 1] CombatInterface X => Floor, Wall, etc
      (set `local.CueTarget` (`self.GetAvatarActorFromActorInfo`))))
  (`GameplayCueFunctionLibrary.AddGameplayCueOnActor` (`local.CueTarget`) (struct :`TagName` "GameplayCue.ChargingLoop") (`self.FirstTargetCueParams`))
  (if (`self.FirstTargetImplementsInterface`)
    (message `CombatInterface.SetIsBeingShocked` (`local.CueTarget`) true)
    (bind _outadditionaltargets (`self.StoreAdditionalTargets`))
    (bind _output_get_2 (set `self.Additional Targets` _outadditionaltargets))
    (for _array_element _output_get_2
      (message `CombatInterface.SetIsBeingShocked` _array_element true)
      (`self.AddChargingLoopCueToAddtionalTarget` _array_element))))

(fn `UpdateFacingTarget`
  (message `CombatInterface.UpdateFacingTarget` (`self.GetAvatarActorFromActorInfo`) (`self.MouseHitLocation`)))