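; Player electric-shot ability that fires a projectile at the mouse target and chains shock damage to nearby targets.
; A montage event spawns the projectile, whose hit delegate is bound through GetActorOfClass.
; On hit, it adds shock cues to chained targets, commits cost, applies SetByCaller magic damage, then cleans up with cooldown.
; Input release can also end it, enforcing minimum time on authority; older looping-beam and damage-timer logic is disconnected.
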(event `Damage And Cost`)

(event `self.K2_ActivateAbility`
  (`self.EnforceImplementsCombatInterface`)
  ;[1 1 1] Store Mouse Data Variables
  (bind (_asynctaskproxy _datahandle) (`TargetDataUnderMouse.CreateTargetDataUnderMouse`)
    (:`ValidData`
      (`self.StoreMouseDataInfo` (`AbilitySystemBlueprintLibrary.GetHitResultFromTargetData` _datahandle))
      (`self.StoreOwnerVariables`)
      (`|ExecutionSequence`
        (:`then_0`
          (`self.UpdateFacingTarget`)
          (`AbilityTask_PlayMontageAndWait.CreatePlayMontageAndWaitProxy` "None" (`self.Montage_Charging`)
            (:`then`
              (`AbilityTask_WaitGameplayEvent.WaitGameplayEvent` (struct :`TagName` "Event.Montage.ElectricShot") null true
                (:`EventReceived`
                  (`self.SpawnProjectile` (`self.MouseHitLocation`) (`BlueprintGameplayTagLibrary.MakeLiteralGameplayTag` (struct :`TagName` "CombatSocket.Weapon")) false 10.0)
                  (bind _returnvalue (`GameplayStatics.GetActorOfClass` (`self.ProjectileClass`)))
                  (`/Engine/EditorBlueprintResources/StandardMacros.IsValid` _returnvalue
                    (:`Is Valid`
                      (add `DreamProjectile.HitActorSignature` _returnvalue (delegate `HitActorSignature_이벤트`)))))))))
        (:`then_1`
          ;[1 1 1] Enforce Minimum Skill Time
          (bind (_asynctaskproxy_2 _timeheld) (`AbilityTask_WaitInputRelease.WaitInputRelease` false)
            (:`OnRelease`
              (bind _output_get (set `self.Time Held` _timeheld))
              (if (< _output_get (`self.MinSkillTime`))
                (`self.K2_HasAuthority`
                  (:`True`
                    (`KismetSystemLibrary.Delay` (- (`self.MinSkillTime`) (`self.Time Held`)))
                    (`self.Clear Timer and End Ability` :!label _label))
                  (:`False`
                    (`self.PrepareForEndAbility`)))
                (else
                  (goto _label))))))))))

(event `HitActorSignature_이벤트`
  (params (TargetActor :type "Actor Object Reference"))
  (set `self.FirstHitActor` TargetActor)
  (bind _output_get (set `self.FirstHitActorCueParams` (`AbilitySystemBlueprintLibrary.MakeGameplayCueParameters` 0.0 0.0 (struct) (struct) (struct) (struct) (struct) (`Actor.K2_GetActorLocation` (`self.FirstHitActor`)))))
  (`GameplayCueFunctionLibrary.AddGameplayCueOnActor` null (struct :`TagName` "GameplayCue.ChargingShot") _output_get)
  (`self.Spawn Electric Effect`)
  (bind _returnvalue (`self.K2_CommitAbilityCost` false))
  (if _returnvalue
    ;[1 1 1] 데미지 적용
    (`self.ApplyDamage`)
    (`KismetSystemLibrary.Delay` 0.2))
  (`self.Clear Timer and End Ability`))

(event `self.PrimaryTargetDied`
  (params (DeadActor :type "Actor Object Reference"))
  ;[1 0.1316 0] PrimaryTargetDied
  (`GameplayCueFunctionLibrary.RemoveGameplayCueOnActor` DeadActor (struct :`TagName` "GameplayCue.ChargingLoop") (`self.FirstTargetCueParams`))
  (`self.K2_CommitAbilityCooldown` false)
  (`self.Clear Timer and End Ability`))

(event `self.AdditionalTargetDied`
  (params (DeadActor :type "Actor Object Reference"))
  ;[1 0.1702 0] Additional Target Died. Remove Additional Targets and Additional ChargingLoop Cue
  (`self.Remove Charging Loop Cue from Additional Target` DeadActor)
  (`KismetArrayLibrary.Array_RemoveItem` (`self.Additional Targets`) DeadActor))

(fn `AddElectricLoopCueToAddtionalTarget`
  (params (AdditionalTarget :type "Actor Object Reference"))
  (locals (TargetActor :type "Actor Object Reference"))
  (bind _targetactor (`local.TargetActor`))
  (bind _returnvalue (`AbilitySystemBlueprintLibrary.MakeGameplayCueParameters` 0.0 0.0 (struct) (struct) (struct) (struct) (struct) (`Actor.K2_GetActorLocation` _targetactor) (0.0 0.0 0.0) null null _targetactor null 1 1 (`Actor.RootComponent` (`self.FirstHitActor`))))
  (set `local.TargetActor` AdditionalTarget)
  (`BlueprintMapLibrary.Map_Add` (`self.AdditionalActorsToCueParams`) (`local.TargetActor`) _returnvalue)
  (`GameplayCueFunctionLibrary.AddGameplayCueOnActor` (`local.TargetActor`) (struct :`TagName` "GameplayCue.ElectricLoop") _returnvalue))

(fn `ApplyDamage`
  ;[1 1 1] Applay Damage to First Hit Actor + Additional Targets
  (`self.ApplyDamageToSingleTarget` (`self.FirstHitActor`))
  (for _array_element (`self.Additional Targets`)
    (`self.ApplyDamageToSingleTarget` _array_element)))

(fn `ApplyDamageToSingleTarget`
  (params (Actor :type "Actor Object Reference"))
  (locals (DamageTarget :type "Actor Object Reference") (ASC :type "AbilitySystemComponent Object Reference"))
  (bind _returnvalue (`self.GetAbilitySystemComponentFromActorInfo`))
  (bind _returnvalue_2 (`AbilitySystemBlueprintLibrary.GetAbilitySystemComponent` (`local.DamageTarget`)))
  (bind _output_get (set `local.DamageTarget` Actor))
  (`/Engine/EditorBlueprintResources/StandardMacros.IsValid` _output_get
    (:`Is Valid`
      (bind _output_get_2 (set `local.ASC` _returnvalue))
      (`/Engine/EditorBlueprintResources/StandardMacros.IsValid` _output_get_2
        (:`Is Valid`
          (bind _returnvalue_3 (`AbilitySystemBlueprintLibrary.AssignTagSetByCallerMagnitude` (`AbilitySystemComponent.MakeOutgoingSpec` (`local.ASC`) (`self.DamageEffectClass`) (`KismetMathLibrary.Conv_IntToDouble` (`self.GetAbilityLevel`)) (`AbilitySystemComponent.MakeEffectContext` _returnvalue)) (struct :`TagName` "Damage.Magical") (`self.GetDamageAtLevel`)))
          (`/Engine/EditorBlueprintResources/StandardMacros.IsValid` _returnvalue_2
            (:`Is Valid`
              (`AbilitySystemComponent.BP_ApplyGameplayEffectSpecToSelf` _returnvalue_2 _returnvalue_3))))))))

(fn `Clear Timer and End Ability`
  (`KismetSystemLibrary.K2_ClearAndInvalidateTimerHandle` (`self.DamageAndCostTimer`))
  (`self.PrepareForEndAbility`)
  (`self.K2_CommitAbilityCooldown` false)
  (`KismetArrayLibrary.Array_Clear` (`self.Additional Targets`))
  (`BlueprintMapLibrary.Map_Clear` (`self.AdditionalActorsToCueParams`))
  (set `self.MouseHitActor` null)
  (set `self.FirstTargetImplementsInterface` false)
  (set `self.Time Held` 0.0)
  (`self.K2_EndAbility`))

(fn `EnforceImplementsCombatInterface`
  (if (not (`KismetSystemLibrary.DoesImplementInterface` (`self.GetAvatarActorFromActorInfo`) "/Script/DreamAdventure.CombatInterface"))
    (`self.K2_EndAbility`)))

(fn `InChargingLoop`
  (message `CombatInterface.SetInCharging` (`self.GetAvatarActorFromActorInfo`) true)
  (`CharacterMovementComponent.DisableMovement` (`Character.CharacterMovement` (`self.OwnerCharacter`))))

(fn `PrepareForEndAbility`
  (bind _firsthitactor (`self.FirstHitActor`))
  (if (`self.FirstTargetImplementsInterface`)
    ;[1 1 1] Case : CombatInterface
    (message `CombatInterface.SetIsBeingShocked` _firsthitactor false)
    (`GameplayCueFunctionLibrary.RemoveGameplayCueOnActor` _firsthitactor (struct :`TagName` "GameplayCue.ElectricLoop") (`self.FirstHitActorCueParams`))
    (`self.K2_HasAuthority`
      (:`True`
        _)
      (:`False`
        _))
    (for _array_element (`self.Additional Targets`)
      (message `CombatInterface.SetIsBeingShocked` _array_element false)
      (`self.Remove Charging Loop Cue from Additional Target` _array_element)
      (`self.K2_HasAuthority`))
    (else
      ;[1 1 1] Case : Wall or Floor .etc for reusing GameplayCue
      (`GameplayCueFunctionLibrary.RemoveGameplayCueOnActor` (`self.GetAvatarActorFromActorInfo`) (struct :`TagName` "GameplayCue.ElectricLoop") (`self.FirstTargetCueParams`)))))

(fn `Remove Charging Loop Cue from Additional Target`
  (params (AddtionalTarget :type "Actor Object Reference"))
  (locals (Target :type "Actor Object Reference"))
  (bind (_value _returnvalue) (`BlueprintMapLibrary.Map_Find` (`self.AdditionalActorsToCueParams`) (`local.Target`)))
  (set `local.Target` AddtionalTarget)
  (if _returnvalue
    _
    (else
      _))
  (`GameplayCueFunctionLibrary.RemoveGameplayCueOnActor` (`local.Target`) (struct :`TagName` "GameplayCue.ElectricLoop") _value))

(fn `Spawn Electric Effect`
  (bind _output_get (set `self.FirstTargetImplementsInterface` (`KismetSystemLibrary.DoesImplementInterface` (`self.FirstHitActor`) "/Script/DreamAdventure.CombatInterface")))
  (if _output_get
    (bind _outadditionaltargets (`self.StoreAdditionalTargets`))
    (bind _output_get_2 (set `self.Additional Targets` _outadditionaltargets))
    (for _array_element _output_get_2
      (message `CombatInterface.SetIsBeingShocked` _array_element true)
      (`self.AddElectricLoopCueToAddtionalTarget` _array_element))))

(fn `SpawnChargingBeam`
  (locals (CueTarget :type "Actor Object Reference"))
  (`self.TraceFirstTarget` (`self.MouseHitLocation`))
  (bind _returnvalue (message `CombatInterface.GetStaticWeapon` (`self.OwnerCharacter`)))
  (set `self.FirstTargetCueParams` (`AbilitySystemBlueprintLibrary.MakeGameplayCueParameters` 0.0 0.0 (struct) (struct) (struct) (struct) (struct) (`self.MouseHitLocation`) (0.0 0.0 0.0) null null (`self.MouseHitActor`) null 1 1 _returnvalue))
  ;[1 1 1] Is Mouse HitActor Enemy?
  (bind _output_get (set `self.FirstTargetImplementsInterface` (`KismetSystemLibrary.DoesImplementInterface` (`self.MouseHitActor`) "/Script/DreamAdventure.CombatInterface")))
  (if _output_get
    ;[1 1 1] CombatInterface => Enemy
    (set `local.CueTarget` (`self.MouseHitActor`))
    (else
      ;[1 1 1] CombatInterface X => Floor, Wall, etc
      (set `local.CueTarget` (`self.GetAvatarActorFromActorInfo`))))
  (`GameplayCueFunctionLibrary.AddGameplayCueOnActor` (`local.CueTarget`) (struct :`TagName` "GameplayCue.ChargingLoop") (`self.FirstTargetCueParams`))
  (if (`self.FirstTargetImplementsInterface`)
    (message `CombatInterface.SetIsBeingShocked` (`local.CueTarget`) true)
    (bind _outadditionaltargets (`self.StoreAdditionalTargets`))
    (bind _output_get_2 (set `self.Additional Targets` _outadditionaltargets))
    (for _array_element _output_get_2
      (message `CombatInterface.SetIsBeingShocked` _array_element true)
      (`self.AddElectricLoopCueToAddtionalTarget` _array_element))))

(fn `UpdateFacingTarget`
  (message `CombatInterface.UpdateFacingTarget` (`self.GetAvatarActorFromActorInfo`) (`self.MouseHitLocation`)))