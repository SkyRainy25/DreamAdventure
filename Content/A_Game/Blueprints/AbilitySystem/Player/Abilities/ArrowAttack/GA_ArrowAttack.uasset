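; GA_ArrowAttack is a player gameplay ability that fires arrow projectiles at the location under the mouse.
; On activation it commits, reads the mouse target data, turns the avatar toward that point and plays a shot montage.
; The montage's gameplay event triggers projectile spawning from the weapon socket, with overridden pitch and the hit actor as homing target.
; The ability ends when the montage completes, is interrupted or is cancelled.
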(event `self.K2_ActivateAbility`
  (`self.K2_CommitAbility`)
  (bind (_asynctaskproxy _datahandle) (`TargetDataUnderMouse.CreateTargetDataUnderMouse`)
    (:`ValidData`
      (bind (_bblockinghit _binitialoverlap _time _distance _location _impactpoint _normal _impactnormal _physmat _hitactor) (`GameplayStatics.BreakHitResult` (`AbilitySystemBlueprintLibrary.GetHitResultFromTargetData` _datahandle)))
      (set `self.Projectile Target Location` _location)
      (set `self.MouseHitActor` _hitactor)
      (message `CombatInterface.UpdateFacingTarget` (`self.GetAvatarActorFromActorInfo`) (`self.Projectile Target Location`))
      (`AbilityTask_PlayMontageAndWait.CreatePlayMontageAndWaitProxy` "None" "/Game/A_Game/Blueprints/Character/Player/ArcherAnimation/AM_Shot_Med2.AM_Shot_Med2" 1.0 "None" false
        (:`then`
          (`AbilityTask_WaitGameplayEvent.WaitGameplayEvent` (struct :`TagName` "Event.Montage.ArrowAttack") null
            (:`EventReceived`
              (`self.SpawnProjectiles` (`self.Projectile Target Location`) (`BlueprintGameplayTagLibrary.MakeLiteralGameplayTag` (struct :`TagName` "CombatSocket.Weapon")) true 10.0 (`self.MouseHitActor`))
              (`KismetSystemLibrary.Delay` 0.5))))
        (:`OnCompleted`
          (`self.K2_EndAbility` :!label _label))
        (:`OnInterrupted`
          (goto _label))
        (:`OnCancelled`
          (goto _label))))))