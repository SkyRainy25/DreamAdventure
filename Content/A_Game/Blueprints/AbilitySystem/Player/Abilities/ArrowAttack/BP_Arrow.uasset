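; BP_Arrow is the arrow actor for the player's ArrowAttack ability, ending in a fire explosion when it stops moving.
; Every Tick, it compares its location with the previous frame's and treats movement at or below MinDistancePerFrame as an impact.
; On impact it spawns a fireball hit sound and a Niagara explosion, then destroys itself.
; No overlap or hit events are used, and the graph applies no damage.
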(event `self.ReceiveTick`
  (params (DeltaSeconds :type "Float (single-precision)"))
  (`self.MakeArrowImpactIfNoMove`))

(fn `MakeArrowImpactIfNoMove`
  (set `self.LocationLastFame` (`self.LocationThisFrame`))
  (set `self.LocationThisFrame` (`self.K2_GetActorLocation`))
  (if (<= (`KismetMathLibrary.VSize` (- (`self.LocationThisFrame`) (`self.LocationLastFame`))) (`self.MinDistancePerFrame`))
    (`GameplayStatics.SpawnSoundAtLocation` "/Game/Assets/Sounds/Abilities/FireBolt/wav/Impact/SFX_Fireball_Hit_01.SFX_Fireball_Hit_01" (`self.LocationThisFrame`) (struct) 1.0 1.0 0.0 null null)
    (`NiagaraFunctionLibrary.SpawnSystemAtLocation` "/Game/Assets/Effects/Projectiles/FireExplosion/NS_FireExplosion.NS_FireExplosion" (`self.LocationThisFrame`))
    (`self.K2_DestroyActor`)))

(fn `UserConstructionScript`)