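; Enemy ranged attack gameplay ability that turns the avatar toward its combat target and fires a projectile at it.
; It plays a random tagged attack montage and waits for that montage's gameplay event tag to time the shot.
; On the event it spawns the projectile from the montage's socket tag toward the target's current location, calls CauseDamage, prints a debug string and ends.
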(event `self.K2_ActivateAbility`
  (bind _returnvalue (`self.GetAvatarActorFromActorInfo`))
  (bind _returnvalue_2 (message `EnemyInterface.GetCombatTarget` _returnvalue))
  (bind _ascombat_interface (cast `CombatInterface` _returnvalue))
  (`CombatInterface.UpdateFacingTarget` _ascombat_interface (`Actor.K2_GetActorLocation` _returnvalue_2))
  (bind _returnvalue_3 (message `CombatInterface.GetAttackMontages` (`self.GetAvatarActorFromActorInfo`)))
  (bind _output_get (set `self.Tagged Montage` (`self.GetRandomTaggedMontageFromArray` _returnvalue_3)))
  (bind (_montage _montagetag) (break `TaggedMontage` _output_get))
  (`AbilityTask_PlayMontageAndWait.CreatePlayMontageAndWaitProxy` "None" _montage
    (:`then`
      (`AbilityTask_WaitGameplayEvent.WaitGameplayEvent` _montagetag null
        (:`EventReceived`
          (message `CombatInterface.GetCombatSocketLocation` (`self.GetAvatarActorFromActorInfo`) _montagetag)
          (bind _returnvalue_4 (message `EnemyInterface.GetCombatTarget` (`self.GetAvatarActorFromActorInfo`)))
          (`self.SpawnProjectile` (`Actor.K2_GetActorLocation` _returnvalue_4) (`.SocketTag` (break `TaggedMontage` (`self.Tagged Montage`))) (`self.Override Pitch`) (`self.Pitch Override`))
          (`self.CauseDamage` null)
          (`KismetSystemLibrary.PrintString` "Hello")
          (`self.K2_EndAbility`))))))