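; Dragon enemy ranged attack ability that fires a volley of projectiles at its combat target.
; On activation it faces the target and plays a random tagged ranged montage, which supplies projectile count and socket tag.
; The montage's gameplay event starts a looping timer that re-reads target location, spawns a projectile and calls CauseDamage on each shot.
; Once the count is reached, it clears the timer, resets the index and ends the ability.
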(event `self.K2_ActivateAbility`
  (bind _returnvalue (`self.GetAvatarActorFromActorInfo`))
  (bind _returnvalue_2 (message `EnemyInterface.GetCombatTarget` _returnvalue))
  (bind _ascombat_interface (cast `CombatInterface` _returnvalue))
  (`CombatInterface.UpdateFacingTarget` _ascombat_interface (`Actor.K2_GetActorLocation` _returnvalue_2))
  (bind _returnvalue_3 (message `CombatInterface.GetRangedAttackMontages` (`self.GetAvatarActorFromActorInfo`)))
  (bind _output_get (set `self.Tagged Montage` (`self.GetRandomTaggedMontageFromArray` _returnvalue_3)))
  (bind (_montage _montagetag _sockettag _impactsound _projectilenum) (break `TaggedMontage` _output_get))
  (set `self.Projectile Num` _projectilenum)
  (set `self.Socket Tag` _sockettag)
  (`AbilityTask_PlayMontageAndWait.CreatePlayMontageAndWaitProxy` "None" _montage
    (:`then`
      (`AbilityTask_WaitGameplayEvent.WaitGameplayEvent` _montagetag null
        (:`EventReceived`
          (bind _returnvalue_4 (message `CombatInterface.GetCombatSocketLocation` (`self.GetAvatarActorFromActorInfo`) _montagetag))
          (set `self.SocketLocation` _returnvalue_4)
          (`self.GetTargetLocation`)
          (bind _returnvalue_5 (`KismetSystemLibrary.K2_SetTimerDelegate` (delegate `커스텀이벤트`) (`self.DelayTime`) true))
          (set `self.Timer` _returnvalue_5))))))

(event `커스텀이벤트`
  (if (< (`self.index`) (`self.Projectile Num`))
    (bind _newparam (`self.GetTargetLocation`))
    (`self.SpawnProjectile` _newparam (`self.Socket Tag`) (`self.Override Pitch`) (`self.Pitch Override`))
    (`self.CauseDamage` null)
    (`/Engine/EditorBlueprintResources/StandardMacros.IncrementInt` (`self.index`))
    (else
      (`KismetSystemLibrary.K2_ClearAndInvalidateTimerHandle` (`self.Timer`))
      (set `self.index` 0)
      (`self.K2_EndAbility`))))

(fn `GetTargetLocation`
  (returns (NewParam :type "Vector Structure"))
  (bind _returnvalue (message `EnemyInterface.GetCombatTarget` (`self.GetAvatarActorFromActorInfo`)))
  (bind _output_get (set `self.TargetLocation` (`Actor.K2_GetActorLocation` _returnvalue)))
  (return _output_get))