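; Boss enemy attack ability that turns to face the combat target and plays a random tagged montage from the avatar's attack montages.
; When the montage's gameplay event arrives, the socket tag selects between a ranged and a close hit.
; The projectile socket fires at a point below the target's location and calls CauseDamage.
; Other sockets damage non-friendly players in a small radius, trigger blood effects and play an impact GameplayCue.
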(event `self.K2_ActivateAbility`
  (bind _returnvalue (`self.GetAvatarActorFromActorInfo`))
  (bind _returnvalue_2 (`self.GetAvatarActorFromActorInfo`))
  (bind _returnvalue_3 (message `EnemyInterface.GetCombatTarget` _returnvalue_2))
  (bind _ascombat_interface (cast `CombatInterface` _returnvalue_2))
  (`CombatInterface.UpdateFacingTarget` _ascombat_interface (`Actor.K2_GetActorLocation` _returnvalue_3))
  (bind _returnvalue_4 (message `CombatInterface.GetAttackMontages` (`self.GetAvatarActorFromActorInfo`)))
  (bind _output_get (set `self.Tagged Montage` (`self.GetRandomTaggedMontageFromArray` _returnvalue_4)))
  (bind (_montage _montagetag _sockettag) (break `TaggedMontage` _output_get))
  (set `self.Socket Tag` _sockettag)
  (`AbilityTask_PlayMontageAndWait.CreatePlayMontageAndWaitProxy` "None" _montage
    (:`then`
      (`AbilityTask_WaitGameplayEvent.WaitGameplayEvent` _montagetag null
        (:`EventReceived`
          (bind _returnvalue_5 (message `CombatInterface.GetCombatSocketLocation` (`self.GetAvatarActorFromActorInfo`) _montagetag))
          (set `self.SocketLocation` _returnvalue_5)
          (if (`BlueprintGameplayTagLibrary.MatchesTag` (`self.Socket Tag`) (struct :`TagName` "CombatSocket.Projectile") true)
            (bind _returnvalue_6 (message `EnemyInterface.GetCombatTarget` (`self.GetAvatarActorFromActorInfo`)))
            (`self.SpawnProjectile` (- (`Actor.K2_GetActorLocation` _returnvalue_6) (0.0 0.0 100.0)) (`self.Socket Tag`) (`self.Override Pitch`) (`self.Pitch Override`))
            (`self.CauseDamage` null)
            (`self.K2_EndAbility`)
            (else
              (bind _outoverlappingactors (`DreamAbilitySystemLibrary.GetLivePlayersWithinRadius` _returnvalue (`|MakeArray` _returnvalue) 50.0 (`self.SocketLocation`)))
              (for _array_element _outoverlappingactors
                (if (`DreamAbilitySystemLibrary.IsNotFriend` (`self.GetAvatarActorFromActorInfo`) _array_element)
                  (`DreamAbilitySystemLibrary.ApplyDamageEffect` (`self.MakeDamageEffectParamsFromClassDefaults` _array_element))
                  (set `self.HasHitTarget` true)
                  (message `CombatInterface.GetBloodEffect` _array_element)))
              (if (`self.HasHitTarget`)
                (message `EnemyInterface.GetCombatTarget` (`self.GetAvatarActorFromActorInfo`))
                (`self.K2_ExecuteGameplayCueWithParams` (struct :`TagName` "GameplayCue.CloseImpact") (`AbilitySystemBlueprintLibrary.MakeGameplayCueParameters` 0.0 0.0 (struct) (struct) (struct) (`BlueprintGameplayTagLibrary.MakeGameplayTagContainerFromTag` (`self.Socket Tag`)) (struct) (`self.SocketLocation`) (0.0 0.0 0.0) null (`self.GetAvatarActorFromActorInfo`)))
                (`self.K2_EndAbility`)
                (else
                  (`self.K2_EndAbility`))))))))))